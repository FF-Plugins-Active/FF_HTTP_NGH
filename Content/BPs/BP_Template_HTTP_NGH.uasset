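; Template Blueprint that starts an HTTP server from the FF_HTTP_NGH plugin when play begins.
; On BeginPlay it looks up the plugin's base directory and builds absolute paths to the bundled web root and 404 page.
; It then spawns an HTTP_Server_NGH actor with those paths, a dynamic API URI and a server name, and keeps a reference to it.
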(event EventBeginPlay
  (bind (_outbasedir _returnvalue) (Class|PluginBlueprintLibrary|GetPluginBaseDir "FF_HTTP_NGH"))
  (if _returnvalue
    (Variables|General|SetPath_Root (Class|BlueprintPathsLibrary|MakePlatformFilename (Class|KismetSystemLibrary|ConverttoAbsolutePath (Utilities|String|Append _outbasedir "/Resources/wwwroot/root/"))))
    (Variables|General|SetPath_404 (Class|KismetSystemLibrary|ConverttoAbsolutePath (Utilities|String|Append _outbasedir "/Resources/wwwroot/404.html"))))
  (bind _returnvalue_2 (Game|SpawnActorfromClass "/Script/FF_HTTP_NGH.HTTP_Server_NGH" (Math|Transform|MakeTransform "0, 0, 0" "0, 0, 0" "1.000000,1.000000,1.000000") "Undefined" "MultiplyWithRoot" 0 (Variables|General|GetPath_Root) (Variables|General|GetPath_404) 8081 8453 "/dyn" "LibWebSocket" 0))
  (Variables|Default|SetServer_NGH _returnvalue_2))

(fn ConstructionScript)